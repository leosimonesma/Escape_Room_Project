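; Test actor for a burn mechanic in which a sphere can be burnt away while lit and later reappears.
; Lighting toggles the lit state, and Burn prints a debug message, hiding the sphere and flagging it burnt only when lit.
; Switching a burnt sphere to unlit starts a timeline that restores visibility and clears the flag on finish.
; Relighting stops that timeline, so the next unlit phase restarts the recovery from zero.
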(event Collision|EventActorBeginOverlap
  (params (OtherActor :type Actor%20Object%20Reference)))

(event EventTick
  (params (DeltaSeconds :type Float%20%28single-precision%29)))

(event EventLighting
  (if (Variables|Default|GetIs_Lighted)
    (Variables|Default|SetIs_Lighted false)
    (if (Variables|Default|GetHas_Been_Burnt)
      (Timeline|Timeline PlayFromStart
        (:Finished
          (Rendering|SetVisibility (Variables|Default|GetSphere) true false)
          (Variables|Default|SetHas_Been_Burnt false))))
    (else
      (Variables|Default|SetIs_Lighted true)
      (Timeline|Timeline Stop))))

(event EventBurn
  (Development|PrintString "Hello")
  (if (Variables|Default|GetIs_Lighted)
    (Rendering|SetVisibility (Variables|Default|GetSphere) false false)
    (Variables|Default|SetHas_Been_Burnt true)))

(event EventBeginPlay)

(fn ConstructionScript)