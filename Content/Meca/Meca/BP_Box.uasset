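; BP_Box is an actor that publishes a box volume's transform to materials through the PC_Box_Data material parameter collection.
; The construction script writes the Sphere component's world location, scale and forward, right and up axes as vector parameters, describing an oriented bounds.
; It has no runtime logic, so the values refresh only when construction reruns, and all instances write to the same collection.
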(event EventBeginPlay)

(event Collision|EventActorBeginOverlap
  (params (OtherActor :type Actor%20Object%20Reference)))

(event EventTick
  (params (DeltaSeconds :type Float%20%28single-precision%29)))

(fn ConstructionScript
  (bind _sphere (Variables|Default|GetSphere))
  (Rendering|Material|SetVectorParameterValue "/Game/Meca/Meca/PC_Box_Data.PC_Box_Data" "Location" (Math|Conversions|ToLinearColor(Vector) (Transformation|GetWorldLocation _sphere)) :!class /Script/Engine.KismetMaterialLibrary)
  (Rendering|Material|SetVectorParameterValue "/Game/Meca/Meca/PC_Box_Data.PC_Box_Data" "Bounds" (Math|Conversions|ToLinearColor(Vector) (Transformation|GetWorldScale _sphere)) :!class /Script/Engine.KismetMaterialLibrary)
  (Rendering|Material|SetVectorParameterValue "/Game/Meca/Meca/PC_Box_Data.PC_Box_Data" "X" (Math|Conversions|ToLinearColor(Vector) (Math|Vector|GetForwardVector _sphere)) :!class /Script/Engine.KismetMaterialLibrary)
  (Rendering|Material|SetVectorParameterValue "/Game/Meca/Meca/PC_Box_Data.PC_Box_Data" "Y" (Math|Conversions|ToLinearColor(Vector) (Math|Vector|GetRightVector _sphere)) :!class /Script/Engine.KismetMaterialLibrary)
  (Rendering|Material|SetVectorParameterValue "/Game/Meca/Meca/PC_Box_Data.PC_Box_Data" "Z" (Math|Conversions|ToLinearColor(Vector) (Math|Vector|GetUpVector _sphere)) :!class /Script/Engine.KismetMaterialLibrary))