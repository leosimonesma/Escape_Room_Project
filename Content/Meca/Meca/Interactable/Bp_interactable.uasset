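; Interactable Blueprint that the player can examine up close, but only while it is lit.
; Lighting toggles the lit state, and BeginPlay pre-creates the examination widget.
; Examine toggles the character's IsLooking flag, blending the view to a camera target and showing the widget after the blend, or blending back to the player and removing it.
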(event EventLighting
  (if (Variables|Default|GetIs_Lighted)
    (Variables|Default|SetIs_Lighted false)
    (else
      (Variables|Default|SetIs_Lighted true))))

(event EventExamine
  (if (Variables|Default|GetIs_Lighted)
    (bind _asbp_third_person_character (Utilities|Casting|CastToBP_ThirdPersonCharacter (Game|GetPlayerCharacter 0)))
    (if (not (Variables|/Game/ThirdPerson/Blueprints/BP_ThirdPersonCharacter.BP_ThirdPersonCharacter_C|Getis%20looking _asbp_third_person_character))
      (Variables|/Game/ThirdPerson/Blueprints/BP_ThirdPersonCharacter.BP_ThirdPersonCharacter_C|Setis%20looking _asbp_third_person_character true)
      (Game|Player|SetViewTargetwithBlend (Game|GetPlayerController 0) (Variables|Default|GetCamera_target) 0.5 "VTBlend_Linear" 0.0 false)
      (Utilities|FlowControl|Delay 0.5)
      (UserInterface|Viewport|AddtoViewport (Variables|Default|GetObjet_01) 0)
      (else
        (Variables|/Game/ThirdPerson/Blueprints/BP_ThirdPersonCharacter.BP_ThirdPersonCharacter_C|Setis%20looking _asbp_third_person_character false)
        (Game|Player|SetViewTargetwithBlend (Game|GetPlayerController 0) (Game|GetPlayerCharacter 0) 0.5 "VTBlend_Linear" 0.0 false)
        (Widget|RemovefromParent (Variables|Default|GetObjet_01))))))

(event EventBeginPlay
  (bind _returnvalue (UserInterface|CreateWidget "/Game/Meca/Widget/WIdget_Interactible_01.WIdget_Interactible_01_C"))
  (Variables|Default|SetObjet_01 _returnvalue))

(fn ConstructionScript)