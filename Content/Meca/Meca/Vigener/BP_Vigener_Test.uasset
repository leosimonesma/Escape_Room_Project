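; Test Blueprint for a Vigenère cipher prototype that generates a random key on BeginPlay.
; ChoixDuChiffre writes a randomly picked ChoixMotChifre entry into NumberMotTest, with a debug print that re-rolls separately.
; BeginPlay then fills MotDuChiffre with one random AlphabetTest character per NumberMotTest element and prints it.
; An unconnected fragment looks up the alphabet index of MsgTest's first letter; no encryption is implemented.
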(event EventBeginPlay
  (bind _mot_du_chiffre (Variables|Default|GetMot_du_chiffre))
  (CallFunction|ChoixDuChiffre)
  ;[1 1 1] Generateur de Clé
  (for (_ _array_index) (Variables|Default|GetNumber_mot_test)
    (Utilities|Array|SetArrayElem _mot_du_chiffre _array_index (Utilities|String|GetSubstring (Variables|Default|GetAlphabet_Test) (Math|Random|RandomIntegerinRange 0 26)) true))
  (for _array_element _mot_du_chiffre
    (Development|PrintString _array_element)))

(event Collision|EventActorBeginOverlap
  (params (OtherActor :type Actor%20Object%20Reference)))

(event EventTick
  (params (DeltaSeconds :type Float%20%28single-precision%29)))

(fn ConstructionScript)

(fn ChoixDuChiffre
  (bind _returnvalue (Math|Random|RandomIntegerinRange 0 10))
  (bind _choix_mot_chifre (LocalVariables|GetChoix_mot_chifre))
  (bind _tableau_10 (Variables|Default|Gettableau_10))
  (bind _returnvalue_2 (Utilities|Array|FindItem _tableau_10 _returnvalue))
  (bind _output (Utilities|Array|Get(acopy) _choix_mot_chifre _returnvalue_2))
  ;[1 1 1] get le bon string a fonction de la génération aléatoire de chiffre
  (for (_array_element _array_index) (Utilities|Array|MakeArray _output)
    (Utilities|Array|SetArrayElem (Variables|Default|GetNumber_mot_test) _array_index _array_element true))
  (Development|PrintString _output))