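; BP_test_light is a test Blueprint that toggles the visibility of its Physic component, apparently as a switchable light.
; The component is hidden on BeginPlay, and the Lighting event flips the IsLighted flag.
; Tick applies that flag to the component's visibility every frame rather than only when it changes.
; Leftover nodes that compare and print Test never run.
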(event EventBeginPlay
  (Rendering|SetVisibility (Variables|Default|GetPhysic) false false))

(event EventTick
  (params (DeltaSeconds :type Float%20%28single-precision%29))
  (bind _physic (Variables|Default|GetPhysic))
  (if (Variables|Default|GetIs_Lighted)
    (Rendering|SetVisibility _physic true false)
    (else
      (Rendering|SetVisibility _physic false false))))

(event EventLighting
  (if (Variables|Default|GetIs_Lighted)
    (Variables|Default|SetIs_Lighted false)
    (else
      (Variables|Default|SetIs_Lighted true))))

(fn ConstructionScript)