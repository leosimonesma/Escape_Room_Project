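; Inspectable item actor that shows proximity interaction icons and opens an inspection view when interacted with.
; ShowIcon toggles the outer icon; ShowInnerInco swaps to the inner icon, which Tick reverts after a short delay unless shown again.
; Interaction, gated by CanInspect, spawns BP_Getting_inspected and passes it the mesh, name, description, rotation and scale.
; The construction script applies the mesh, scale, sphere radii and debug sphere visibility.
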(event EventBeginPlay
  (Transformation|SetRelativeLocation (Variables|Default|GetInner_Icon) (Variables|Instance_editable|Icon_Parameter|GetInner_Icon_Location) false false)
  (Transformation|SetRelativeLocation (Variables|Default|GetOuter_Icon) (Variables|Instance_editable|Icon_Parameter|GetOuter_Icon_Location) false false))

(event EventTick
  (params (DeltaSeconds :type Float%20%28single-precision%29))
  ;[1 1 1] Interaction icon visibility
  (if (Variables|Bool|GetInner)
    (Utilities|FlowControl|Delay 0.1)
    (Rendering|SetVisibility (Variables|Default|GetInner_Icon) false false)
    (Rendering|SetVisibility (Variables|Default|GetOuter_Icon) true false)
    (Variables|Bool|SetInner false)))

(event EventShowIcon
  (bind _outer_icon (Variables|Default|GetOuter_Icon))
  ;[1 1 1] Interaction icon visibility
  (if (Variables|Bool|GetOuter)
    (Rendering|SetVisibility _outer_icon false false)
    (Variables|Bool|SetOuter false)
    (else
      (Rendering|SetVisibility _outer_icon true false)
      (Variables|Bool|SetOuter true))))

(event EventShowInnerInco
  ;[1 1 1] Interaction icon visibility
  (if (not (Variables|Bool|GetInner))
    (Rendering|SetVisibility (Variables|Default|GetInner_Icon) true false)
    (Rendering|SetVisibility (Variables|Default|GetOuter_Icon) false false)
    (Variables|Bool|SetInner true)))

(event EventInteraction
  (params (Interactor :type BP%20Third%20Person%20Character%20Object%20Reference))
  (if (Variables|Instance_editable|Bool|GetCan_Inspect?)
    (bind _returnvalue (Game|SpawnActorfromClass "/Game/Meca/BP/inspectable/BP_Getting_inspected.BP_Getting_inspected_C" (Math|Transform|MakeTransform "300.000000,0.000000,0.000000") "Undefined" "MultiplyWithRoot" 0 0))
    (Default|SetInspectRotation _returnvalue (Variables|Instance_editable|Inspection_parameter|GetInspection_Rotation))
    (Default|SetInspectScale _returnvalue (Variables|Instance_editable|Inspection_parameter|GetInspection_Scale))
    (Class|BPILightingObject|Inspection(Message) _returnvalue Interactor (Variables|/Script/Engine.StaticMeshComponent|GetStaticMesh (Variables|Default|GetStaticMesh)) (Variables|Instance_editable|Item_Parameter|GetItem_Name) (Variables|Instance_editable|Item_Parameter|GetItem_Description))))

(fn ConstructionScript
  (bind _staticmesh (Variables|Default|GetStaticMesh))
  (bind _sphere_outer (Variables|Default|GetSphere_Outer))
  (bind _sphere_inner (Variables|Default|GetSphere_Inner))
  (Utilities|FlowControl|Sequence
    (:then_0
      ;[1 1 1] Setting Sphère collision radius
      (Components|Sphere|SetSphereRadius (Variables|Default|GetSphere_Inner) (Variables|Instance_editable|Icon_Parameter|GetInner_Sphere_Radius) true)
      (Components|Sphere|SetSphereRadius (Variables|Default|GetSphere_Outer) (Variables|Instance_editable|Icon_Parameter|GetOuter_Sphere_Radius) true))
    (:then_1
      ;[1 1 1] set Mesh
      (Components|StaticMesh|SetStaticMesh (Variables|Default|GetStaticMesh) (Variables|Instance_editable|Item_Parameter|GetItem_Mesh))
      ;[1 1 1] set scale
      (Transformation|SetWorldTransform _staticmesh (Math|Transform|MakeTransform (Transformation|GetWorldLocation _staticmesh) (Transformation|GetWorldRotation _staticmesh) (Variables|Instance_editable|Item_Parameter|GetItem_Scale)) false false))
    (:then_2
      ;[1 1 1] voir les radius pour du debbug
      (if (Variables|Instance_editable|Icon_Parameter|GetIs_Debbuging%20?%20)
        (Rendering|SetVisibility _sphere_inner true false)
        (Rendering|SetVisibility _sphere_outer true false)
        (else
          (Rendering|SetVisibility _sphere_inner false false)
          (Rendering|SetVisibility _sphere_outer false false))))))