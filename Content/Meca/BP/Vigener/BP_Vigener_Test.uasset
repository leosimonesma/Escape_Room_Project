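; Test Blueprint for a Vigenère cipher puzzle that prepares a random word and key on BeginPlay, printing the results for debugging.
; ChoixDuChiffre copies a number-word array (Zero to Six) into MotDuChiffre, re-evaluating the random pick at each branch; higher-number branches are unwired.
; A same-length key is drawn from AlphabetTest, and each letter's Alphabet index is stored in StockIndex.
; No encryption step exists yet.
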(event EventBeginPlay
  (bind _mot_du_chiffre (Variables|Default|GetMot_du_chiffre))
  (CallFunction|ChoixDuChiffre)
  (Development|PrintString "mdc" true true "(R=0.000000,G=0.660000,B=1.000000,A=1.000000)" 4e+01)
  (for _array_element _mot_du_chiffre
    (Development|PrintString _array_element true true "(R=0.000000,G=0.660000,B=1.000000,A=1.000000)" 4e+01))
  ;[1 1 1] Generateur de Clé
  (for (_ _array_index) _mot_du_chiffre
    (Utilities|Array|SetArrayElem (Variables|Default|Getclé) _array_index (Utilities|String|GetSubstring (Variables|Default|GetAlphabet_Test) (Math|Random|RandomIntegerinRange 0 26)) true))
  (Development|PrintString "clé" true true "(R=0.000000,G=0.660000,B=1.000000,A=1.000000)" 4e+01)
  (for _array_element_2 (Variables|Default|Getclé)
    (Development|PrintString _array_element_2 true true "(R=0.000000,G=0.660000,B=1.000000,A=1.000000)" 4e+01))
  ;[1 1 1] Gader en mémoire l'index des lettres
  (for (_array_element_3 _array_index_2) (Variables|Default|GetMot_du_chiffre)
    (bind _output_get (Variables|Default|SetIndex_memory (Utilities|Array|FindItem (Variables|Default|GetAlphabet) (Utilities|String|GetSubstring _array_element_3 0))))
    (Utilities|Array|SetArrayElem (Variables|Default|GetStock_index) _array_index_2 _output_get true))
  (Development|PrintString "index" true true "(R=0.000000,G=0.660000,B=1.000000,A=1.000000)" 4e+01)
  (for _array_element_4 (Variables|Default|GetStock_index)
    (Development|PrintString (Utilities|String|ToString(Integer) _array_element_4) true true "(R=0.000000,G=0.660000,B=1.000000,A=1.000000)" 4e+01))
  (Development|PrintString "fin" true true "(R=0.000000,G=0.660000,B=1.000000,A=1.000000)" 4e+01))

(event Collision|EventActorBeginOverlap
  (params (OtherActor :type Actor%20Object%20Reference)))

(event EventTick
  (params (DeltaSeconds :type Float%20%28single-precision%29)))

(fn ConstructionScript)

(fn ChoixDuChiffre
  (bind _random (LocalVariables|Getrandom))
  (bind _outindex (Utilities|Array|Random _random))
  (Development|PrintString "random" true true "(R=0.000000,G=0.660000,B=1.000000,A=1.000000)" 4e+01)
  (Development|PrintString (Utilities|String|ToString(Integer) _outindex) true true "(R=0.000000,G=0.660000,B=1.000000,A=1.000000)" 4e+01)
  (if (== _outindex 0)
    (for (_array_element _array_index) (LocalVariables|Getzero)
      (Utilities|Array|SetArrayElem (Variables|Default|GetMot_du_chiffre) _array_index _array_element true))
    (elif (== _outindex 1)
      (for (_array_element_2 _array_index_2) (LocalVariables|Getun)
        (Utilities|Array|SetArrayElem (Variables|Default|GetMot_du_chiffre) _array_index_2 _array_element_2 true))
      (elif (== _outindex 2)
        (for (_array_element_3 _array_index_3) (LocalVariables|Getdeux)
          (Utilities|Array|SetArrayElem (Variables|Default|GetMot_du_chiffre) _array_index_3 _array_element_3 true))
        (elif (== _outindex 3)
          (for (_array_element_4 _array_index_4) (LocalVariables|Gettrois)
            (Utilities|Array|SetArrayElem (Variables|Default|GetMot_du_chiffre) _array_index_4 _array_element_4 true))
          (elif (== _outindex 4)
            (for (_array_element_5 _array_index_5) (LocalVariables|Getquatre)
              (Utilities|Array|SetArrayElem (Variables|Default|GetMot_du_chiffre) _array_index_5 _array_element_5 true))
            (elif (== _outindex 5)
              (for (_array_element_6 _array_index_6) (LocalVariables|Getcinq)
                (Utilities|Array|SetArrayElem (Variables|Default|GetMot_du_chiffre) _array_index_6 _array_element_6 true))
              (elif (== _outindex 6)
                (for (_array_element_7 _array_index_7) (LocalVariables|Getsix)
                  (Utilities|Array|SetArrayElem (Variables|Default|GetMot_du_chiffre) _array_index_7 _array_element_7 true))))))))))