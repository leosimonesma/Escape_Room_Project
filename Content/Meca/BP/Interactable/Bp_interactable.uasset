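; Interactable actor that the third-person player can examine up close, but only while its IsLighted flag is on.
; The Lighting event flips that flag, and Examine toggles the character's IsLooking state.
; Examining blends the view to CameraTarget, then after a short delay shows a widget pre-created at BeginPlay and calls the character's ShowMouse.
; Examining again blends back to the player, removes the widget and calls ShowMouse again.
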(event EventLighting
  (Development|PrintString "Hello")
  (if (Variables|Default|GetIs_Lighted)
    (Variables|Default|SetIs_Lighted false)
    (else
      (Variables|Default|SetIs_Lighted true))))

(event EventExamine
  (Development|PrintString "Hello")
  (if (Variables|Default|GetIs_Lighted)
    (bind _asbp_third_person_character (Utilities|Casting|CastToBP_ThirdPersonCharacter (Game|GetPlayerCharacter 0)))
    (Variables|Default|SetAs%20BP%20Third%20Person%20Character _asbp_third_person_character)
    (if (not (Variables|/Game/ThirdPerson/Blueprints/BP_ThirdPersonCharacter.BP_ThirdPersonCharacter_C|Getis%20looking (Variables|Default|GetAs%20BP%20Third%20Person%20Character)))
      (Variables|/Game/ThirdPerson/Blueprints/BP_ThirdPersonCharacter.BP_ThirdPersonCharacter_C|Setis%20looking (Variables|Default|GetAs%20BP%20Third%20Person%20Character) true)
      (Game|Player|SetViewTargetwithBlend (Game|GetPlayerController 0) (Variables|Default|GetCamera_target) 0.5 "VTBlend_Linear" 0.0 false)
      (Utilities|FlowControl|Delay 0.5)
      (UserInterface|Viewport|AddtoViewport (Variables|Default|GetObjet_01) 0)
      (Default|ShowMouse (Variables|Default|GetAs%20BP%20Third%20Person%20Character))
      (else
        (Variables|/Game/ThirdPerson/Blueprints/BP_ThirdPersonCharacter.BP_ThirdPersonCharacter_C|Setis%20looking (Variables|Default|GetAs%20BP%20Third%20Person%20Character) false)
        (Game|Player|SetViewTargetwithBlend (Game|GetPlayerController 0) (Game|GetPlayerCharacter 0) 0.5 "VTBlend_Linear" 0.0 false)
        (Widget|RemovefromParent (Variables|Default|GetObjet_01))
        (Default|ShowMouse (Variables|Default|GetAs%20BP%20Third%20Person%20Character))))))

(event EventBeginPlay
  (bind _returnvalue (UserInterface|CreateWidget "/Game/Meca/Widget/BPI_WIdget_Interactible_01.BPI_WIdget_Interactible_01_C"))
  (Variables|Default|SetObjet_01 _returnvalue))

(fn ConstructionScript)