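; BP_Radio is an interactable item, named as a radio, with two interaction icons and an optional inspection view.
; The construction script sets its mesh, scale and inner and outer sphere radii, with a debug flag showing the spheres.
; ShowIcon and ShowInnerInco toggle the icons on each call.
; When Inspect is set, Interaction spawns a BP_inspectable and passes it the interactor, mesh, name, description and inspection rotation and scale.
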(event EventBeginPlay
  (|CallParentFunction)
  (Transformation|SetRelativeLocation (Variables|Default|GetOuter_Interact_Icon) (Variables|Instance_editable|settings|Geticon_location_Outer) false false)
  (Transformation|SetRelativeLocation (Variables|Default|GetInner_Interact_Icon) (Variables|Instance_editable|settings|GetIcon_location_intter) false false))

(event Collision|EventActorBeginOverlap
  (params (OtherActor :type Actor%20Object%20Reference))
  (|CallParentFunction OtherActor) ; This node is disabled and will not be called.\nDrag off pins to build functionality.
)

(event EventTick
  (params (DeltaSeconds :type Float%20%28single-precision%29))
  (|CallParentFunction DeltaSeconds) ; This node is disabled and will not be called.\nDrag off pins to build functionality.
)

(event EventShowIcon
  ;[1 1 1] Interaction icon visibility
  (if (Variables|Default|GetOuter)
    (Rendering|SetVisibility (Variables|Default|GetOuter_Interact_Icon) false false)
    (Variables|Default|SetOuter false)
    (else
      (Rendering|SetVisibility (Variables|Default|GetOuter_Interact_Icon) true false)
      (Variables|Default|SetOuter true))))

(event EventInteraction
  (params (Interactor :type BP%20Third%20Person%20Character%20Object%20Reference))
  ;[1 1 1] creation du widget pour inspecter avec les bonnes ref
  (if (Variables|Instance_editable|inspection|GetInspect?)
    (bind _returnvalue (Game|SpawnActorfromClass "/Game/Meca/BP/inspectable/BP_inspectable.BP_inspectable_C" (Math|Transform|MakeTransform "300.000000,0.000000,0.000000") "Undefined" "MultiplyWithRoot" 0 0))
    (Default|SetInspectRotation _returnvalue (Variables|InstanceEditable|Inspection|GetItem_inspection_rotation))
    (Default|SetInspectScale _returnvalue (Variables|InstanceEditable|Inspection|GetItem_inspection_Scale))
    (Class|BPILightingObject|Inspection(Message) _returnvalue Interactor (Variables|/Script/Engine.StaticMeshComponent|GetStaticMesh (Variables|Default|GetStatic_Mesh)) (Variables|Instance_editable|Ref|GetItem_name) (Variables|Instance_editable|Ref|GetItem_description))))

(event EventShowInnerInco
  ;[1 1 1] Interaction icon visibility
  (if (Variables|Default|Getinner)
    (Rendering|SetVisibility (Variables|Default|GetInner_Interact_Icon) false false)
    (Rendering|SetVisibility (Variables|Default|GetOuter_Interact_Icon) true false)
    (Variables|Default|Setinner false)
    (else
      (Rendering|SetVisibility (Variables|Default|GetInner_Interact_Icon) true false)
      (Rendering|SetVisibility (Variables|Default|GetOuter_Interact_Icon) false false)
      (Variables|Default|Setinner true))))

(fn ConstructionScript
  (bind _outer_sphere_collision (Variables|Default|GetOuter_Sphere_Collision))
  (bind _inner_sphere_collision (Variables|Default|GetInner_Sphere_Collision))
  (bind _static_mesh (Variables|Default|GetStatic_Mesh))
  (|CallParentFunction)
  (Utilities|FlowControl|Sequence
    (:then_0
      ;[1 1 1] Setting Sphère collision radius
      (Components|Sphere|SetSphereRadius (Variables|Default|GetInner_Sphere_Collision) (Variables|InstanceEditable|Settings|GetInner_Sphere_Radius) true)
      (Components|Sphere|SetSphereRadius (Variables|Default|GetOuter_Sphere_Collision) (Variables|InstanceEditable|Settings|GetOuter_Sphere_Radius) true))
    (:then_1
      ;[1 1 1] set Mesh
      (Components|StaticMesh|SetStaticMesh (Variables|Default|GetStatic_Mesh) (Variables|Instance_editable|Ref|GetItem_Mesh))
      ;[1 1 1] set scale
      (Transformation|SetWorldTransform _static_mesh (Math|Transform|MakeTransform (Transformation|GetWorldLocation _static_mesh) (Transformation|GetWorldRotation _static_mesh) (Variables|Instance_editable|Ref|GetItem_scale)) false false))
    (:then_2
      ;[1 1 1] voir les radius pour du debbug
      (if (Variables|InstanceEditable|Settings|GetDebbugin?)
        (Rendering|SetVisibility _inner_sphere_collision true false)
        (Rendering|SetVisibility _outer_sphere_collision true false)
        (else
          (Rendering|SetVisibility _inner_sphere_collision false false)
          (Rendering|SetVisibility _outer_sphere_collision false false))))))