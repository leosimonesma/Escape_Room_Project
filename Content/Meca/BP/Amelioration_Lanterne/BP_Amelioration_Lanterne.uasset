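; Lantern upgrade pickup that grants the player character either the first or second light, depending on its ID.
; BeginPlay caches the character and builds the matching message widget.
; Examine grants the light, shows the message for a few seconds while hiding the mesh, then destroys the actor.
; ShowIcon toggles the outer prompt icon, while ShowInnerInco swaps to the inner icon, which Tick reverts after a short delay.
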(event EventBeginPlay
  ;[1 1 1] set up des widgets messages
  (bind _asbp_third_person_character (Utilities|Casting|CastToBP_ThirdPersonCharacter (Game|GetPlayerCharacter 0)))
  (Variables|Default|SetAs%20BP%20Third%20Person%20Character _asbp_third_person_character)
  (if (== (Variables|ID|GetID) 0)
    (bind _returnvalue (UserInterface|CreateWidget "/Game/Meca/Widget/WB_Getting_Light.WB_Getting_Light_C" 0 (Variables|Messages|GetMessage_First_light) (Variables|Messages|GetMessage_Getting_light)))
    (Variables|Default|SetFirst_Light _returnvalue)
    (else
      (bind _returnvalue_2 (UserInterface|CreateWidget "/Game/Meca/Widget/WB_Getting_Light.WB_Getting_Light_C" 0 (Variables|Messages|GetMessage_Second_light) (Variables|Messages|GetMessage_Getting_light) (Variables|Messages|GetSwitch_Lights)))
      (Variables|Default|SetSecond_Light _returnvalue_2))))

(event EventTick
  (params (DeltaSeconds :type Float%20%28single-precision%29))
  ;[1 1 1] icon visibility
  (if (Variables|Default|Getinner)
    (Utilities|FlowControl|Delay 0.1)
    (Rendering|SetVisibility (Variables|Default|GetInner_Icon) false false)
    (Rendering|SetVisibility (Variables|Default|GetOuter_Icon) true false)
    (Variables|Default|SetInner false)))

(event EventExamine
  ;[1 1 1] récuperation des amélioration
  (if (== (Variables|ID|GetID) 0)
    (Default|SetFirstLight (Variables|Default|GetAs%20BP%20Third%20Person%20Character))
    (UserInterface|Viewport|AddtoViewport (Variables|Default|GetFirst_Light) 0)
    (Rendering|SetVisibility (Variables|Default|GetStaticMesh) false false)
    (Utilities|FlowControl|Delay 5.0)
    (Widget|RemovefromParent (Variables|Default|GetFirst_Light))
    (else
      (Default|SetSecondLight (Variables|Default|GetAs%20BP%20Third%20Person%20Character))
      (UserInterface|Viewport|AddtoViewport (Variables|Default|GetSecond_Light) 0)
      (Rendering|SetVisibility (Variables|Default|GetStaticMesh) false false)
      (Utilities|FlowControl|Delay 5.0)
      (Widget|RemovefromParent (Variables|Default|GetSecond_Light))))
  (Actor|DestroyActor self))

(event EventShowIcon
  (bind _outer_icon (Variables|Default|Getouter_icon))
  ;[1 1 1] icon visibility
  (if (Variables|Default|GetOuter)
    (Rendering|SetVisibility _outer_icon false false)
    (Variables|Default|SetOuter false)
    (else
      (Rendering|SetVisibility _outer_icon true false)
      (Variables|Default|SetOuter true))))

(event EventShowInnerInco
  ;[1 1 1] icon visibility
  (if (not (Variables|Default|Getinner))
    (Rendering|SetVisibility (Variables|Default|GetInner_Icon) true false)
    (Rendering|SetVisibility (Variables|Default|GetOuter_Icon) false false)
    (Variables|Default|SetInner true)
    (Development|PrintString "Hello")))

(fn ConstructionScript)