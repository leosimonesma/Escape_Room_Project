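; BP_Burn is an actor whose mesh can be burnt away while lit and returns some time after it is unlit.
; Burn, if IsLighted, hides the mesh, ignores Pawn and Camera collision and flags HasBeenBurnt, after a debug print.
; Lighting toggles IsLighted: unlighting a burnt mesh starts a Timeline used as a delay, relighting stops it.
; When the Timeline finishes, visibility and Pawn blocking return, but Camera stays ignored.
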(event EventBeginPlay
  (|CallParentFunction) ; This node is disabled and will not be called.\nDrag off pins to build functionality.
)

(event Collision|EventActorBeginOverlap
  (params (OtherActor :type Actor%20Object%20Reference))
  (|CallParentFunction OtherActor) ; This node is disabled and will not be called.\nDrag off pins to build functionality.
)

(event EventTick
  (params (DeltaSeconds :type Float%20%28single-precision%29))
  (|CallParentFunction DeltaSeconds) ; This node is disabled and will not be called.\nDrag off pins to build functionality.
)

(event EventLighting
  (if (Variables|Default|GetIs_Lighted)
    (Variables|Default|SetIs_Lighted false)
    (if (Variables|Default|GetHas_Been_Burnt)
      (Timeline|Timeline PlayFromStart
        (:Finished
          (Rendering|SetVisibility (Variables|Default|GetStaticMesh) true false)
          (Collision|SetCollisionResponsetoChannel (Variables|Default|GetStaticMesh) "ECC_Pawn" "ECR_Block")
          (Variables|Default|SetHas_Been_Burnt false))))
    (else
      (Variables|Default|SetIs_Lighted true)
      (Timeline|Timeline Stop))))

(event EventBurn
  (Development|PrintString "Hello")
  (if (Variables|Default|GetIs_Lighted)
    (Rendering|SetVisibility (Variables|Default|GetStaticMesh) false false)
    (Collision|SetCollisionResponsetoChannel (Variables|Default|GetStaticMesh) "ECC_Pawn" "ECR_Ignore")
    (Collision|SetCollisionResponsetoChannel (Variables|Default|GetStaticMesh) "ECC_Camera" "ECR_Ignore")
    (Variables|Default|SetHas_Been_Burnt true)))

(fn ConstructionScript
  (|CallParentFunction))