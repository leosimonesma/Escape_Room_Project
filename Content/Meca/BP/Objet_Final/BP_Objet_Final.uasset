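; BP_Objet_Final is the final-object actor that displays the end screen widget, WB_Fin.
; It creates the widget on BeginPlay and keeps it in a variable, then adds it to the viewport when its Fin event is called.
; An unconnected chain for moving a box and blending to a camera before the screen appears remains in the graph but never runs.
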(event Custom|Fin
  (UserInterface|Viewport|AddtoViewport (Variables|Default|GetNewVar) 0))

(event EventBeginPlay
  (bind _returnvalue (UserInterface|CreateWidget "/Game/Meca/Widget/WB_Fin.WB_Fin_C"))
  (Variables|Default|SetNewVar _returnvalue))

(fn ConstructionScript)