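; BP_Lock is a puzzle lock that plays the Secretaire animation once solved.
; It creates a WB_Lock widget at BeginPlay, and a Lighting event toggles whether it can be examined.
; Examine toggles the player's looking state, blending between CameraTarget and the character while adding or removing the widget and calling ShowMouse.
; The widget's solved flag is read only on exiting the view, then blocks further examination.
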(event EventBeginPlay
  (|CallParentFunction)
  (bind _returnvalue (UserInterface|CreateWidget "/Game/Meca/Widget/WB_Lock.WB_Lock_C"))
  (Variables|Default|SetNewVar_0 _returnvalue))

(event Collision|EventActorBeginOverlap
  (params (OtherActor :type Actor%20Object%20Reference))
  (|CallParentFunction OtherActor) ; This node is disabled and will not be called.\nDrag off pins to build functionality.
)

(event EventTick
  (params (DeltaSeconds :type Float%20%28single-precision%29))
  (|CallParentFunction DeltaSeconds) ; This node is disabled and will not be called.\nDrag off pins to build functionality.
)

(event EventExamine
  (if (and (Variables|Default|GetIs_Lighted) (not (Variables|Default|GetIs_Solved)))
    (bind _asbp_third_person_character (Utilities|Casting|CastToBP_ThirdPersonCharacter (Game|GetPlayerCharacter 0)))
    (Variables|Default|SetAs%20BP%20Third%20Person%20Character _asbp_third_person_character)
    (if (not (Variables|/Game/ThirdPerson/Blueprints/BP_ThirdPersonCharacter.BP_ThirdPersonCharacter_C|Getis%20looking (Variables|Default|GetAs%20BP%20Third%20Person%20Character)))
      (Variables|/Game/ThirdPerson/Blueprints/BP_ThirdPersonCharacter.BP_ThirdPersonCharacter_C|Setis%20looking (Variables|Default|GetAs%20BP%20Third%20Person%20Character) true)
      (Game|Player|SetViewTargetwithBlend (Game|GetPlayerController 0) (Variables|Default|GetCamera_target) 0.5 "VTBlend_Linear" 0.0 false)
      (Utilities|FlowControl|Delay 0.5)
      (UserInterface|Viewport|AddtoViewport (Variables|Default|GetNewVar_0) 0)
      (Default|ShowMouse (Variables|Default|GetAs%20BP%20Third%20Person%20Character))
      (else
        (Variables|/Game/ThirdPerson/Blueprints/BP_ThirdPersonCharacter.BP_ThirdPersonCharacter_C|Setis%20looking (Variables|Default|GetAs%20BP%20Third%20Person%20Character) false)
        (Game|Player|SetViewTargetwithBlend (Game|GetPlayerController 0) (Game|GetPlayerCharacter 0) 0.5 "VTBlend_Linear" 0.0 false)
        (Widget|RemovefromParent (Variables|Default|GetNewVar_0))
        (Default|ShowMouse (Variables|Default|GetAs%20BP%20Third%20Person%20Character))
        (if (Variables|/Game/Meca/Widget/WB_Lock.WB_Lock_C|GetIs_Solved (Variables|Default|GetNewVar_0))
          (Variables|Default|SetIs_Solved true)
          (Components|Animation|PlayAnimation (Variables|Default|Getsecretaire) "/Game/Props/Mesh/Meubles/Secretaire/secretaire_Anim.secretaire_Anim" false))))))

(event EventLighting
  (if (Variables|Default|GetIs_Lighted)
    (Variables|Default|SetIs_Lighted false)
    (else
      (Variables|Default|SetIs_Lighted true))))

(fn ConstructionScript
  (|CallParentFunction))