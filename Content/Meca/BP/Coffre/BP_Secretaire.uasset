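; BP_Secretaire is an examinable secretary desk with a lock puzzle, usable only while lit and unsolved.
; Examine toggles the player's looking state, blending the view to the desk camera and showing the WB_Lock widget created at BeginPlay.
; On exit it restores the player view, removes the widget and, if the lock is solved, marks itself solved and plays the desk's animation.
; The Lighting event toggles the lit state.
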(event EventBeginPlay
  (bind _returnvalue (UserInterface|CreateWidget "/Game/Meca/Widget/WB_Lock.WB_Lock_C"))
  (Variables|Ref|SetWidget_ref _returnvalue))

(event EventExamine
  (Development|PrintString "Hello")
  (if (and (Variables|Bool|GetIs_Lighted) (not (Variables|Bool|GetIs_Solved)))
    (bind _asbp_third_person_character (Utilities|Casting|CastToBP_ThirdPersonCharacter (Game|GetPlayerCharacter 0)))
    (Variables|Ref|SetAs%20BP%20Third%20Person%20Character _asbp_third_person_character)
    (if (not (Variables|/Game/ThirdPerson/Blueprints/BP_ThirdPersonCharacter.BP_ThirdPersonCharacter_C|Getis%20looking (Variables|Ref|GetAs%20BP%20Third%20Person%20Character)))
      (Variables|/Game/ThirdPerson/Blueprints/BP_ThirdPersonCharacter.BP_ThirdPersonCharacter_C|Setis%20looking (Variables|Ref|GetAs%20BP%20Third%20Person%20Character) true)
      (Game|Player|SetViewTargetwithBlend (Game|GetPlayerController 0) (Variables|Ref|GetCamera_Ref) 0.5 "VTBlend_Linear" 0.0 false)
      (Utilities|FlowControl|Delay 0.5)
      (UserInterface|Viewport|AddtoViewport (Variables|Ref|GetWidget_ref) 0)
      (Default|ShowMouse (Variables|Ref|GetAs%20BP%20Third%20Person%20Character))
      (else
        (Variables|/Game/ThirdPerson/Blueprints/BP_ThirdPersonCharacter.BP_ThirdPersonCharacter_C|Setis%20looking (Variables|Ref|GetAs%20BP%20Third%20Person%20Character) false)
        (Game|Player|SetViewTargetwithBlend (Game|GetPlayerController 0) (Game|GetPlayerCharacter 0) 0.5 "VTBlend_Linear" 0.0 false)
        (Widget|RemovefromParent (Variables|Ref|GetWidget_ref))
        (Default|ShowMouse (Variables|Ref|GetAs%20BP%20Third%20Person%20Character))
        (if (Variables|/Game/Meca/Widget/WB_Lock.WB_Lock_C|GetIs_Solved (Variables|Ref|GetWidget_ref))
          (Variables|Bool|SetIs_Solved true)
          (Components|Animation|PlayAnimation (Variables|Default|Getsecretaire) "/Game/Props/Mesh/Meubles/Secretaire/secretaire_Anim.secretaire_Anim" false))))))

(event EventLighting
  (if (Variables|Bool|GetIs_Lighted)
    (Variables|Bool|SetIs_Lighted false)
    (else
      (Variables|Bool|SetIs_Lighted true))))

(fn ConstructionScript)